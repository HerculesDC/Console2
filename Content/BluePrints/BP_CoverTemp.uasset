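; BP_CoverTemp is a cover actor that tells TPSCharacters when they stand in one of its two cover volumes, Front or Back.
; Overlapping a volume sets the character's OverlappingCoverVolume to it, and leaving clears the reference only if it still points to that volume.
; BeginPlay stores the ChildActorComponents as CoverSpots, and an unconnected debug loop would print CoverSpotV2 states.
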(event OnComponentBeginOverlap(Back)
  (params (OverlappedComponent :type Primitive%20Component%20Object%20Reference) (OtherActor :type Actor%20Object%20Reference) (OtherComp :type Primitive%20Component%20Object%20Reference) (OtherBodyIndex :type Integer) (bFromSweep :type Boolean) (SweepResult :type Hit%20Result%20Structure%20%28by%20ref%29))
  (CallFunction|TakeCover OtherActor (Variables|Default|GetBack)))

(event OnComponentEndOverlap(Back)
  (params (OverlappedComponent :type Primitive%20Component%20Object%20Reference) (OtherActor :type Actor%20Object%20Reference) (OtherComp :type Primitive%20Component%20Object%20Reference) (OtherBodyIndex :type Integer))
  (CallFunction|LeaveCover OtherActor (Variables|Default|GetBack)))

(event OnComponentBeginOverlap(Front)
  (params (OverlappedComponent :type Primitive%20Component%20Object%20Reference) (OtherActor :type Actor%20Object%20Reference) (OtherComp :type Primitive%20Component%20Object%20Reference) (OtherBodyIndex :type Integer) (bFromSweep :type Boolean) (SweepResult :type Hit%20Result%20Structure%20%28by%20ref%29))
  (CallFunction|TakeCover OtherActor (Variables|Default|GetFront)))

(event OnComponentEndOverlap(Front)
  (params (OverlappedComponent :type Primitive%20Component%20Object%20Reference) (OtherActor :type Actor%20Object%20Reference) (OtherComp :type Primitive%20Component%20Object%20Reference) (OtherBodyIndex :type Integer))
  (CallFunction|LeaveCover OtherActor (Variables|Default|GetFront)))

(event Custom|TakeCover
  (params (OverlappedActor :type Actor%20Object%20Reference) (OverlappingVolume :type Box%20Component%20Object%20Reference))
  (bind _astpscharacter (Utilities|Casting|CastToTPSCharacter OverlappedActor))
  (Variables|/Script/ThirdPersonShooter.TPSCharacter|SetoverlappingCoverVolume _astpscharacter OverlappingVolume))

(event Custom|LeaveCover
  (params (OverlappedActor :type Actor%20Object%20Reference) (OverlappingVolume :type Box%20Component%20Object%20Reference))
  (bind _astpscharacter (Utilities|Casting|CastToTPSCharacter OverlappedActor))
  (if (== (Variables|/Script/ThirdPersonShooter.TPSCharacter|GetoverlappingCoverVolume _astpscharacter) OverlappingVolume)
    (Variables|/Script/ThirdPersonShooter.TPSCharacter|SetoverlappingCoverVolume _astpscharacter 0)))

(event EventBeginPlay
  (Variables|Default|SetCoverSpots (Actor|GetComponentsByClass "/Script/Engine.ChildActorComponent")))

(event Collision|EventActorBeginOverlap
  (params (OtherActor :type Actor%20Object%20Reference)))

(event EventTick
  (params (DeltaSeconds :type Float%20%28single-precision%29)))

(fn ConstructionScript)